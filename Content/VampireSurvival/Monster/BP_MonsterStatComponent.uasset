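; Monster stat component for the VampireSurvival game that holds a monster's current stats and HP and handles damage and death.
; SetMonStat loads a row from DT_Monster, starts current HP at the row's MaxHP and broadcasts the new stats.
; AddDamage ignores monsters that are already dead, otherwise subtracts HP and fires the HP update dispatcher, plus the death dispatcher when HP drops below one.
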(fn `AddDamage`
  (params (Damage :type "Float (double-precision)"))
  (bind (_curmonsterstat_mondata _curmonsterstat_curhp) (break `/Game/VampireSurvival/Monster/ST_CurMonster` (`self.CurMonsterStat`)))
  (bind _curmonsterstat (`self.CurMonsterStat`))
  (if (not (`self.IsDeath`))
    (bind _structout (setmembers `/Game/VampireSurvival/Monster/ST_CurMonster` :`StructRef` (`self.CurMonsterStat`) :`CurHP` (- _curmonsterstat_curhp Damage)))
    (`self.EventDispatcher_UpdateHP` (`.CurHP_5_E9F474CE44E5E432C043B0A13DFA3AE6` (break `/Game/VampireSurvival/Monster/ST_CurMonster` _curmonsterstat)) (`.MaxHP_9_C19834FE4D09D4A7DDFAE8AB3FC0B895` (break `/Game/VampireSurvival/Monster/ST_Monster` (break `/Game/VampireSurvival/Monster/ST_CurMonster` _curmonsterstat))))
    (if (< (`.CurHP_5_E9F474CE44E5E432C043B0A13DFA3AE6` (break `/Game/VampireSurvival/Monster/ST_CurMonster` _structout)) 1.0)
      (`self.EventDispatcher_Death` (`self.CurMonsterStat`)))))

(fn `IsDeath`
  (returns (IsJustDeath :type Boolean))
  (bind (_curmonsterstat_mondata _curmonsterstat_curhp) (break `/Game/VampireSurvival/Monster/ST_CurMonster` (`self.CurMonsterStat`)))
  (return (< _curmonsterstat_curhp 1.0)))

(fn `SetMonStat`
  (params (RowName :type Name))
  (bind _returnvalue (`|GetDataTableRow` "/Game/VampireSurvival/Monster/DT_Monster.DT_Monster" RowName)
    (:`then`
      (bind _output_get (set `self.CurMonsterStat` (make `/Game/VampireSurvival/Monster/ST_CurMonster` _returnvalue (`.MaxHP_9_C19834FE4D09D4A7DDFAE8AB3FC0B895` (break `/Game/VampireSurvival/Monster/ST_Monster` _returnvalue)))))
      (`self.EventDispatcher_MonsterStat` _output_get))))