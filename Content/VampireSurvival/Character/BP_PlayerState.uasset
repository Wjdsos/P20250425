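; BP_PlayerState tracks the player's health in the VampireSurvival game.
; AddDamage subtracts damage from current HP unless the player is already dead, then broadcasts an Update dispatcher with current and max HP.
; When HP drops below one it fires a Death dispatcher, using the same threshold that IsDeath reports.
; The event graph and construction script are empty.
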(fn `AddDamage`
  (params (Damage :type "Float (double-precision)"))
  (if (not (`self.IsDeath`))
    (bind _output_get (set `self.CurHP` (- (`self.CurHP`) Damage)))
    (`self.EventDispatcher_Update` _output_get (`self.MaxHP`))
    (if (< (`self.CurHP`) 1.0)
      (`self.EventDispatcher_Death`))))

(fn `IsDeath`
  (returns (IsJustDeath :type Boolean))
  (return (< (`self.CurHP`) 1.0)))

(fn `UserConstructionScript`)