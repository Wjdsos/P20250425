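; BP_Slash is a slash skill actor in the VampireSurvival game that deals one burst of area damage around the character that uses it.
; On BeginPlay it snaps onto that Character's mesh in position and rotation while keeping world scale.
; It then immediately applies radial damage at its own location, ignoring the Character and crediting its controller as instigator.
; The graph has no tick, repeat hit or cleanup logic.
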(event `self.ReceiveBeginPlay`
  (`self.K2_AttachToComponent` (`Character.Mesh` (`self.Character`)) "None" "SnapToTarget" "SnapToTarget" "KeepWorld")
  (`GameplayStatics.ApplyRadialDamage` 20.0 (`self.K2_GetActorLocation`) 200.0 null (`|MakeArray` (`self.Character`) :!type "Actor Object Reference") self (`Pawn.GetController` (`self.Character`))))

(fn `UserConstructionScript`
  (`parent.UserConstructionScript`))